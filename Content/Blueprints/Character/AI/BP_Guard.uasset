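; BP_Guard is an AI guard character Blueprint that layers weapon and hit-reaction setup on top of its parent class.
; On BeginPlay it calls the parent, then has EquipmentComponent attach the weapon to the hand.
; Physical animation setup and hit reaction events are forwarded to PhysicalAnimComp.
; PostCombatStateEnabled is empty, and the idle-to-combat montage node is left unconnected, so it never plays.
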(event EventBeginPlay
  (|CallParentFunction)
  (Class|EquipmentComponent|AttachWeapontoHand (Variables|Default|GetEquipmentComponent)))

(event Collision|EventActorBeginOverlap
  (params (OtherActor :type Actor%20Object%20Reference))
  (|CallParentFunction OtherActor) ; This node is disabled and will not be called.\nDrag off pins to build functionality.
)

(event EventSetupPhysicalAnimation
  (Default|SetUpPhysicalAnimation (Variables|Default|GetPhysicalAnimComp)))

(event EventPostCombatStateEnabled)

(event EventTick
  (params (DeltaSeconds :type Float%20%28single-precision%29))
  (|CallParentFunction DeltaSeconds) ; This node is disabled and will not be called.\nDrag off pins to build functionality.
)

(event EventHitReaction
  (params (HitResult :type Hit%20Result%20Structure))
  (Default|HitReaction (Variables|Default|GetPhysicalAnimComp) HitResult))

(fn ConstructionScript
  (|CallParentFunction))