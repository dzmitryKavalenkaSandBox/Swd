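; Player character Blueprint that handles touch camera rotation and keyboard-triggered melee attacks.
; Touch movement feeds scaled position deltas into controller yaw and pitch, resetting the start pose each event.
; X, Z and E keys each assign a kick or swing attack to AttackComponent, then execute it.
; Sphere-trace lock-on targeting and input-mode setup are present but disconnected, so they never run.
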(event Custom|UpdatePose
  (params (UpdatePose :type Vector%202D%20Structure))
  (bind _startpose (Variables|Default|GetStartPose))
  (bind _returnvalue (- UpdatePose _startpose))
  (bind _returnvalue_2 (/ _returnvalue 5.0))
  ;[1 1 1] Touch rotate camera
  (Pawn|Input|AddControllerYawInput (.x _returnvalue_2))
  (Pawn|Input|AddControllerPitchInput (.y _returnvalue_2)))

(event EventBeginPlay)

(event Input|ActionEvents|InputActionLockOn
  (params (Key :type Key%20Structure :default "None")))

(event Input|KeyboardEvents|Z
  (params (Key :type Key%20Structure :default "None"))
  (bind _attackcomponent (Variables|Default|GetAttackComponent))
  (:Pressed
    (Class|AttackComponent|SetAttacktoPerform _attackcomponent "/Game/Blueprints/Character/Attacks/BP_LeftLegKickAttack.BP_LeftLegKickAttack_C")
    (Class|AttackComponent|Attack _attackcomponent)))

(event Input|KeyboardEvents|X
  (params (Key :type Key%20Structure :default "None"))
  (bind _attackcomponent (Variables|Default|GetAttackComponent))
  (:Pressed
    (Class|AttackComponent|SetAttacktoPerform _attackcomponent "/Game/Blueprints/Character/Attacks/BP_RightLegKickAttack.BP_RightLegKickAttack_C")
    (Class|AttackComponent|Attack _attackcomponent)))

(event Input|KeyboardEvents|E
  (params (Key :type Key%20Structure :default "None"))
  (bind _attackcomponent (Variables|Default|GetAttackComponent))
  (:Pressed
    (Class|AttackComponent|SetAttacktoPerform _attackcomponent "/Game/Blueprints/Character/Attacks/BP_FastSwingFromRight.BP_FastSwingFromRight_C")
    (Class|AttackComponent|Attack _attackcomponent)))

(event Input|TouchEvents|InputTouch
  (params (Location :type Vector) (FingerIndex :type ETouchIndex%20Enum))
  (bind (_x _y) (Math|Vector|BreakVector Location))
  ;[1 1 1] Touch rotate camera
  (:Pressed
    (Variables|Default|SetStartPose (Math|Vector2D|MakeVector2D _x _y) :!label _label))
  (:Released
    (goto _label))
  (:Moved
    (CallFunction|UpdatePose (Math|Vector2D|MakeVector2D _x _y))
    (goto _label)))

(fn ConstructionScript)