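; Character component that plays physics-driven hit reactions on an SwdCharacter's skeletal mesh.
; A setup event adds a PhysicalAnimationComponent to the owner and binds it to the mesh.
; Hits simulate bodies below the pelvis with the HitReactionProfile, apply a directional impulse to the struck bone (spine for pelvis hits) and extend a timer.
; Tick decays that timer as the physics blend weight, then disables simulation, ticking and physics collision.
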(event Custom|Set%20Up%20Physical%20Animation
  (bind _returnvalue (Components|GetOwner))
  (bind _returnvalue_2 (Game|AddComponentbyClass _returnvalue "/Script/Engine.PhysicalAnimationComponent"))
  (bind _output_get (Variables|Default|SetPhyscal%20Animation%20Component _returnvalue_2))
  (bind _asswd_character (Utilities|Casting|CastToSwdCharacter _returnvalue))
  (Class|PhysicalAnimationComponent|SetSkeletalMeshComponent _output_get (Variables|/Script/Engine.Character|GetMesh _asswd_character))
  (Variables|Default|SetMesh (Variables|/Script/Engine.Character|GetMesh _asswd_character)))

(event Custom|TogglePhysAnim
  (Collision|SetCollisionEnabled (Variables|Default|GetMesh) "QueryAndPhysics")
  (Class|SkeletalMeshComponent|SetAllBodiesBelowSimulatePhysics (Variables|Default|GetMesh) (Utilities|Name|MakeLiteralName "pelvis") true false)
  (Class|PhysicalAnimationComponent|ApplyPhysicalAnimationProfileBelow (Variables|Default|GetPhyscal%20Animation%20Component) "pelvis" "HitReactionProfile" false false))

(event Custom|Hit%20Reaction
  (params (Hit :type Hit%20Result%20Structure))
  (bind (_bblockinghit _binitialoverlap _time _distance _location _impactpoint _normal _impactnormal _physmat _hitactor _hitcomponent _hitbonename _bonename _hititem _elementindex _faceindex _tracestart _traceend) (Collision|BreakHitResult Hit))
  (Collision|SetCollisionEnabled (Variables|Default|GetMesh) "QueryAndPhysics")
  (Components|Tick|SetComponentTickEnabled true)
  (Variables|Default|SetHit%20Raction%20Time%20Remaining (+ (Variables|Default|GetHit%20Raction%20Time%20Remaining) 2.0))
  (Class|PhysicalAnimationComponent|ApplyPhysicalAnimationProfileBelow (Variables|Default|GetPhyscal%20Animation%20Component) "pelvis" "HitReactionProfile" false false)
  (Class|SkeletalMeshComponent|SetAllBodiesBelowSimulatePhysics (Variables|Default|GetMesh) (Utilities|Name|MakeLiteralName "pelvis") true false)
  (Physics|AddImpulse (Variables|Default|GetMesh) (* (Math|Vector|Normalize (- _traceend _tracestart)) 5e+04) (select (== _hitbonename "pelvis") (Utilities|Name|MakeLiteralName "spine_01") _hitbonename) true))

(event EventBeginPlay)

(event EventTick
  (params (DeltaSeconds :type Float%20%28single-precision%29))
  (Variables|Default|SetHit%20Raction%20Time%20Remaining (- (Math|Interpolation|FInterpTo (Variables|Default|GetHit%20Raction%20Time%20Remaining) 0.0 0.0 1.0) (* DeltaSeconds 0.8)))
  (if (<= (Variables|Default|GetHit%20Raction%20Time%20Remaining) 0.0)
    (Variables|Default|SetHit%20Raction%20Time%20Remaining 0.0)
    (Class|SkeletalMeshComponent|SetAllBodiesBelowSimulatePhysics (Variables|Default|GetMesh) (Utilities|Name|MakeLiteralName "pelvis") false true)
    (Components|Tick|SetComponentTickEnabled false)
    (Collision|SetCollisionEnabled (Variables|Default|GetMesh) "QueryOnly")
    (else
      (Class|SkeletalMeshComponent|SetAllBodiesBelowPhysicsBlendWeight (Variables|Default|GetMesh) (Utilities|Name|MakeLiteralName "pelvis") (Math|Float|Min(Float) (Variables|Default|GetHit%20Raction%20Time%20Remaining) 1.0) false true))))